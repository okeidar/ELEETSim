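; BP_TestPlatform is an operable test interaction object that shows its on/off state through the color of a point light.
; StartOperate sets the On flag and turns the light blue, while StopOperate clears the flag and turns it red.
; BeginPlay colors the light from the initial On value, and IsOperating reports that flag to callers.
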(event EventBeginPlay
  (Rendering|Components|Light|SetLightColor (Variables|Default|GetPointLight) (Math|Color|SelectColor "(R=0.000000,G=0.000000,B=1.000000,A=1.000000)" "(R=1.000000,G=0.000000,B=0.000000,A=1.000000)" (Variables|Default|GetbOn)) true))

(event EventStartOperate
  (Rendering|Components|Light|SetLightColor (Variables|Default|GetPointLight) "(R=0.000000,G=0.000000,B=1.000000,A=1.000000)" true)
  (Variables|Default|SetbOn true))

(event EventStopOperate
  (Rendering|Components|Light|SetLightColor (Variables|Default|GetPointLight) "(R=1.000000,G=0.000000,B=0.000000,A=1.000000)" true)
  (Variables|Default|SetbOn false))

(fn ConstructionScript)

(fn IsOperating
  (return (Variables|Default|GetbOn)))